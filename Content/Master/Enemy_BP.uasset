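; Enemy AI character that fights the player's ninja with sword attacks, strafing and parries.
; On seeing the ninja through PawnSensing, a weighted roll picks either approach-and-attack or a short back, left or right strafe.
; The approach equips the sword if needed and repeats until in range, then plays a random attack.
; Tick turns the enemy toward its target during attacks and strafes, applying strafe movement and random parrying.
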(event `ShowBar`
  (params (`show?` :type Boolean))
  (`SceneComponent.SetVisibility` (`self.Widget`) `show?` false))

(event `Show Decal`
  (params (`show?` :type Boolean))
  (`SceneComponent.SetVisibility` (`self.Decal`) `show?` false))

(event `self.PawnSensing.OnSeePawn`
  (params (Pawn :type "Pawn Object Reference"))
  (if (not (`self.has target?`))
    (bind _asninja_bp (cast `/Game/Master/Ninja_BP` Pawn))
    (bind _output_get (set `self.Target` _asninja_bp))
    (set `self.has target?` true)
    (set `self.enemy attacking?` false)
    (switch `int` (`KismetMathLibrary.Conv_BoolToInt` (`KismetMathLibrary.RandomBoolWithWeight` (`self.Enemy Attack Weight`)))
      (:`0`
        (`|AIMoveTo` self (0.0 0.0 0.0) _output_get 150.0 :!label _label
          (:`then`
            (if (not (`self.SwordEquipped?`))
              (`self.EquipSword`)
              (`KismetSystemLibrary.Delay` 0.5))
            (`KismetSystemLibrary.Delay` 0.4)
            (if (< (`self.GetDistanceTo` (`GameplayStatics.GetPlayerCharacter` 0)) 220.0)
              (set `self.AttackNr` (`KismetMathLibrary.RandomIntegerInRange` 0 2))
              (`self.Enemy Attack`)
              (set `self.enemy attacking?` true)
              (`KismetSystemLibrary.Delay` 0.9)
              (set `self.has target?` false)
              (set `self.Ready?` true)
              (set `self.enemy attacking?` false)
              (else
                (goto _label))))))
      (:`1`
        (set `self.enemy attacking?` false)
        (set `self.is strafing?` true)
        (switch `int` (`KismetMathLibrary.RandomIntegerInRange` 0 2)
          (:`0`
            (set `self.Strafe` "NewEnumerator0"))
          (:`1`
            (set `self.Strafe` "NewEnumerator1"))
          (:`2`
            (set `self.Strafe` "NewEnumerator2")))
        (`KismetSystemLibrary.Delay` 0.5)
        (set `self.is strafing?` false)
        (set `self.has target?` false)))))

(event `self.ReceiveTick`
  (params (DeltaSeconds :type "Float (single-precision)"))
  (bind (_returnvalue_roll _returnvalue_pitch) (`KismetMathLibrary.BreakRotator` (`self.K2_GetActorRotation`)))
  (bind (_returnvalue_roll_2 _returnvalue_pitch_2) (`KismetMathLibrary.BreakRotator` (`self.K2_GetActorRotation`)))
  (bind _target (`self.Target`))
  (bind _target_2 (`self.Target`))
  (bind (_returnvalue_roll_3 _returnvalue_pitch_3 _returnvalue_yaw) (`KismetMathLibrary.BreakRotator` (`KismetMathLibrary.FindLookAtRotation` (`self.K2_GetActorLocation`) (`self.K2_GetActorLocation` _target_2))))
  (bind (_returnvalue_roll_4 _returnvalue_pitch_4 _returnvalue_yaw_2) (`KismetMathLibrary.BreakRotator` (`KismetMathLibrary.FindLookAtRotation` (`self.K2_GetActorLocation`) (`self.K2_GetActorLocation` _target))))
  (`parent.ReceiveTick` DeltaSeconds)
  (if (`self.has target?`)
    (if (`self.enemy attacking?`)
      (`/Engine/EditorBlueprintResources/StandardMacros.IsValid` _target_2
        (:`Is Valid`
          (`self.K2_SetActorRotation` (`KismetMathLibrary.MakeRotator` _returnvalue_roll _returnvalue_pitch _returnvalue_yaw))))
      (elif (`self.is strafing?`)
        (`/Engine/EditorBlueprintResources/StandardMacros.IsValid` _target
          (:`Is Valid`
            (`self.K2_SetActorRotation` (`KismetMathLibrary.MakeRotator` _returnvalue_roll_2 _returnvalue_pitch_2 _returnvalue_yaw_2))
            (`self.AddMovementInput` (`self.Strafing`))
            (if (`KismetMathLibrary.RandomBoolWithWeight` 0.5)
              (`self.Enemy Parrying` true))))
        (else
          (`self.Enemy Parrying` false))))))

(fn `Strafing`
  (returns (`Strafing Direction Vector` :type "Vector Structure"))
  (bind _returnvalue (`self.GetActorRightVector`))
  (switch `/Game/Master/AI/Strafe_Direction` (`self.Strafe`)
    (:`NewEnumerator0`
      (set `self.Strafing Direction Vector` (* (`self.GetActorForwardVector`) -1.0)))
    (:`NewEnumerator1`
      (set `self.Strafing Direction Vector` _returnvalue))
    (:`NewEnumerator2`
      (set `self.Strafing Direction Vector` (* _returnvalue -1.0))))
  (return (`self.Strafing Direction Vector`)))

(fn `UserConstructionScript`
  (`parent.UserConstructionScript`))